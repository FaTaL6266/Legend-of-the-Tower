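; Builder ghost actor that previews tower placement and spawns the real tower.
; Each tick it snaps the cursor's world-static hit to a 100-unit grid at fixed height.
; A downward line trace for pawns sets whether building is allowed and swaps the ghost mesh between green and red translucent materials.
; PlaceTower, when allowed, spawns TowerBP, passes it the tower data, initializes it, then destroys the ghost.
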(event `self.ReceiveBeginPlay`)

(event `self.ReceiveTick`
  (params (DeltaSeconds :type "Float (single-precision)"))
  (bind _ghostmesh (`self.GhostMesh`))
  (bind (_hitresult _returnvalue) (`PlayerController.GetHitResultUnderCursorForObjects` (`GameplayStatics.GetPlayerController` 0) (`|MakeArray` "ObjectTypeQuery1" :!type "EObjectTypeQuery Enum") true))
  (bind _returnvalue_2 (`PrimitiveComponent.GetMaterial` _ghostmesh 0))
  (if _returnvalue
    (bind _output_get (set `self.SnapLocation` (`KismetMathLibrary.MakeVector` (`KismetMathLibrary.GridSnap_Float` (.x (`.Location` (`GameplayStatics.BreakHitResult` _hitresult))) 100.0) (`KismetMathLibrary.GridSnap_Float` (.y (`.Location` (`GameplayStatics.BreakHitResult` _hitresult))) 100.0) 167.0)))
    (bind (_outhit _returnvalue_3) (`KismetSystemLibrary.LineTraceSingleForObjects` :`Start` (+ _output_get (0.0 0.0 300.0)) :`End` _output_get :`ObjectTypes` (`|MakeArray` "ObjectTypeQuery3" :!type "EObjectTypeQuery Enum") :`DrawDebugType` "ForOneFrame"))
    (if _returnvalue_3
      (set `self.CanBuild` false)
      (if (not (== _returnvalue_2 "/Game/Tower/RedTranslucent.RedTranslucent"))
        (`PrimitiveComponent.SetMaterial` _ghostmesh 0 "/Game/Tower/RedTranslucent.RedTranslucent"))
      (else
        (set `self.CanBuild` true)
        (if (not (== _returnvalue_2 "/Game/Tower/GreenTranslucent.GreenTranslucent"))
          (`PrimitiveComponent.SetMaterial` _ghostmesh 0 "/Game/Tower/GreenTranslucent.GreenTranslucent"))))
    (`self.K2_SetActorLocation` (`self.SnapLocation`))))

(event `PlaceTower`
  (if (`self.CanBuild`)
    (bind _returnvalue (`|SpawnActorFromClass` "/Game/Tower/TowerBP.TowerBP_C" (`self.GetTransform`) "AlwaysSpawn" "OverrideRootScale" null null))
    (set `/Game/Tower/TowerBP.TowerStruct` (`self.TowerData`) _returnvalue)
    (`/Game/Tower/TowerBP.TowerInit` _returnvalue)
    (`self.K2_DestroyActor`)))

(fn `UserConstructionScript`)